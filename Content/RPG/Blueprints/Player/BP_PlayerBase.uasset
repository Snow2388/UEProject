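; BP_PlayerBase is the RPG player character, handling Enhanced Input movement, camera turning and weapon pickup.
; Overlapping an object leads to WuQiShiQu, which detaches the held weapon, attaches the new sword, axe or bow to its socket and routes input to it; axes slow walking.
; XiuZheng provides aim correction, sphere-tracing pawns and snapping yaw toward the nearest eligible enemy, with persistent debug drawing left on.
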(event `self.ReceiveBeginPlay`
  ;[1 1 1] 添加输入映射
  (bind _asbp_play_controller (cast `/Game/RPG/Blueprints/BP_PlayController` (`self.GetController`)))
  (bind _returnvalue (pcsubsystem `EnhancedInputLocalPlayerSubsystem` _asbp_play_controller))
  (`/Engine/EditorBlueprintResources/StandardMacros.IsValid` _returnvalue
    (:`Is Valid`
      (`EnhancedInputSubsystemInterface.AddMappingContext` _returnvalue "/Game/RPG/Input/IMC_Default.IMC_Default" 0 (struct)))))

(event `EnhancedInput|/Game/RPG/Input/IA/IA_Move`
  (params (ActionValue :type "Vector2D Structure") (ElapsedSeconds :type "Float (double-precision)") (TriggeredSeconds :type "Float (double-precision)") (InputAction :type "InputAction Object Reference" :default "/Game/RPG/Input/IA/IA_Move.IA_Move"))
  (bind (_returnvalue_roll _returnvalue_pitch _returnvalue_yaw) (`KismetMathLibrary.BreakRotator` (`self.GetControlRotation`)))
  ;[1 1 1] 移动
  (:`Triggered`
    (`self.AddMovementInput` (`KismetMathLibrary.GetRightVector` (`KismetMathLibrary.MakeRotator` 0.0 0.0 _returnvalue_yaw)) ActionValue_X)
    (`self.AddMovementInput` (`KismetMathLibrary.GetForwardVector` (`KismetMathLibrary.MakeRotator` 0.0 0.0 _returnvalue_yaw)) ActionValue_Y)))

(event `EnhancedInput|/Game/RPG/Input/IA/IA_Turn`
  (params (ActionValue :type "Vector2D Structure") (ElapsedSeconds :type "Float (double-precision)") (TriggeredSeconds :type "Float (double-precision)") (InputAction :type "InputAction Object Reference" :default "/Game/RPG/Input/IA/IA_Turn.IA_Turn"))
  ;[1 1 1] 旋转视角
  (:`Triggered`
    (bind _asbp_play_controller (cast `/Game/RPG/Blueprints/BP_PlayController` (`GameplayStatics.GetPlayerController` 0)))
    (`PlayerController.AddYawInput` _asbp_play_controller ActionValue_X)
    (`PlayerController.AddPitchInput` _asbp_play_controller ActionValue_Y)))

(event `self.ShiQu.OnComponentBeginOverlap`
  (params (OverlappedComponent :type "PrimitiveComponent Object Reference") (OtherActor :type "Actor Object Reference") (OtherComp :type "PrimitiveComponent Object Reference") (OtherBodyIndex :type Integer) (bFromSweep :type Boolean) (SweepResult :type "HitResult Structure (by ref)"))
  ;[1 1 1] 拾取武器
  (bind _asbp_object_base (cast `/Game/RPG/Blueprints/BP_ObjectBase` OtherActor))
  (switch `/Game/RPG/DataType/E_ObjectType` (`/Game/RPG/Blueprints/BP_ObjectBase.ObjectType` _asbp_object_base)
    (:`NewEnumerator0`
      (`self.WuQiShiQu` _asbp_object_base))))

(fn `UserConstructionScript`)

(fn `WuQiShiQu`
  (params (WuQi :type "Actor Object Reference"))
  (locals (Socket_WuQi :type Name :default "None"))
  (bind _wuqi_shou (`self.WuQi_Shou`))
  (bind _asbp_wu_qi_base (cast `/Game/RPG/Blueprints/WuQi/BP_WuQiBase` WuQi))
  (`/Engine/EditorBlueprintResources/StandardMacros.IsValid` _wuqi_shou
    (:`Is Valid`
      (`self.K2_DetachFromActor` _wuqi_shou "KeepWorld" "KeepWorld" "KeepWorld")
      (set `CharacterMovementComponent.MaxWalkSpeed` 600.0 (`self.CharacterMovement`))
      (`self.DisableInput` _wuqi_shou (`GameplayStatics.GetPlayerController` 0))
      (set `/Game/RPG/Blueprints/WuQi/BP_WuQiBase.User` null _wuqi_shou))
    (:`Is Not Valid`
      _))
  (bind _output_get (set `self.WuQi_Shou` _asbp_wu_qi_base))
  (set `/Game/RPG/Blueprints/WuQi/BP_WuQiBase.User` self _output_get)
  (switch `/Game/RPG/DataType/E_WuQiType` (`/Game/RPG/Blueprints/WuQi/BP_WuQiBase.WuQiType` _output_get)
    (:`NewEnumerator1`
      (set `local.Socket_WuQi` "Jian"))
    (:`NewEnumerator2`
      (set `CharacterMovementComponent.MaxWalkSpeed` 350.0 (`self.CharacterMovement`))
      (set `local.Socket_WuQi` "FuTou"))
    (:`NewEnumerator3`
      (set `local.Socket_WuQi` "Gong")))
  (`self.K2_AttachToComponent` (`self.WuQi_Shou`) (`self.Mesh`) (`local.Socket_WuQi`) "SnapToTarget" "SnapToTarget" "SnapToTarget" true)
  (`self.EnableInput` (`self.WuQi_Shou`) (`GameplayStatics.GetPlayerController` 0)))

(fn `XiuZheng`
  (params (XiuZhengFanWei :type "Float (double-precision)"))
  (locals (MinJuLi :type "Float (double-precision)") (MinEnemy :type "/Game/RPG/Blueprints/Enemy/BP_EnemyBase Object Reference"))
  (bind (_returnvalue_roll _returnvalue_pitch) (`KismetMathLibrary.BreakRotator` (`self.K2_GetActorRotation`)))
  (bind _returnvalue (`self.K2_GetActorLocation`))
  (bind (_returnvalue_roll_2 _returnvalue_pitch_2 _returnvalue_yaw) (`KismetMathLibrary.BreakRotator` (`KismetMathLibrary.FindLookAtRotation` (`self.K2_GetActorLocation`) (`self.K2_GetActorLocation` (`local.MinEnemy`)))))
  (bind _output_get (set `local.MinJuLi` XiuZhengFanWei))
  (bind (_outhits _returnvalue_2) (`KismetSystemLibrary.SphereTraceMultiForObjects` :`Start` _returnvalue :`End` _returnvalue :`Radius` _output_get :`ObjectTypes` (`|MakeArray` "ObjectTypeQuery3" :!type "EObjectTypeQuery Enum") :`DrawDebugType` "Persistent"))
  (if _returnvalue_2
    (for _array_element _outhits
      (bind (_bblockinghit _binitialoverlap _time _distance _location _impactpoint _normal _impactnormal _physmat _hitactor) (`GameplayStatics.BreakHitResult` _array_element))
      (bind _returnvalue_3 (`self.GetDistanceTo` _hitactor))
      ;[1 1 1 0.3] 寻找最近敌人
      (if (< _returnvalue_3 (`local.MinJuLi`))
        (bind _asbp_enemy_base (cast `/Game/RPG/Blueprints/Enemy/BP_EnemyBase` _hitactor))
        (if (`|EnumInequality` (`/Game/RPG/Blueprints/Enemy/BP_EnemyBase.State` _asbp_enemy_base) "NewEnumerator3")
          (set `local.MinEnemy` _asbp_enemy_base)
          (set `local.MinJuLi` _returnvalue_3))))
    ;[1 1 1 0.3] 修正朝向最近敌人
    (`local.MinEnemy`
      (:`then`
        (`self.K2_SetActorRotation` (`KismetMathLibrary.MakeRotator` _returnvalue_roll _returnvalue_pitch _returnvalue_yaw)))
      (:`else`))))