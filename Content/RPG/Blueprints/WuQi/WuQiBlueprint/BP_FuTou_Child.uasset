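; Axe weapon child Blueprint that plays a two-section combo attack montage on its user when the attack input triggers.
; A DoOnce gates each swing, starting AM_FuTou_A at the current section and disabling the user's input.
; StartGongJi extends the parent's version, advancing the section index with wraparound and reopening the gate.
; Montage completion resets the combo index and gate and re-enables the user's input.
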(event `self.ReceiveBeginPlay`
  (`parent.ReceiveBeginPlay`)
  (set `self.AMPianDuan` (`|MakeArray` "0" "1" :!type "Name")))

(event `GongJiAM`
  (`/Engine/EditorBlueprintResources/StandardMacros.DoOnce` false :!label _label
    (:`Completed`
      (`|PlayMontage` (`Character.Mesh` (`self.User`)) "/Game/RPG/Animation/GongJi/AM_FuTou_A.AM_FuTou_A" 1.0 0.0 (`|GetArrayItem` (`self.AMPianDuan`) (`self.NowPianDuanIndex`))
        (:`then`
          (`self.DisableInput` (`self.User`) (`GameplayStatics.GetPlayerController` 0)))
        (:`OnCompleted`
          (set `self.NowPianDuanIndex` 0)
          (`self.EnableInput` (`self.User`) (`GameplayStatics.GetPlayerController` 0))
          (`self.Reset`))))))

(event `Reset`
  (goto _label :!via `Reset`))

(event `EnhancedInput|/Game/RPG/Input/IA/IA_GongJi`
  (params (ActionValue :type Boolean) (ElapsedSeconds :type "Float (double-precision)") (TriggeredSeconds :type "Float (double-precision)") (InputAction :type "InputAction Object Reference" :default "/Game/RPG/Input/IA/IA_GongJi.IA_GongJi"))
  (:`Triggered`
    (`self.GongJiAM`)))

(fn `StartGongJi`
  (`parent.StartGongJi`)
  (bind _result (`/Engine/EditorBlueprintResources/StandardMacros.IncrementInt` (`self.NowPianDuanIndex`))
    (:`  `
      (if (not (`KismetArrayLibrary.Array_IsValidIndex` (`self.AMPianDuan`) _result))
        (set `self.NowPianDuanIndex` 0))
      (`self.Reset`))))

(fn `UserConstructionScript`
  (`parent.UserConstructionScript`))