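; Bow weapon child Blueprint that plays the user's attack montage and provides functions to spawn and fire arrows.
; The attack input passes a DoOnce gate, calls XiuZheng on the user, and plays an indexed montage section, disabling player input until completion resets the gate.
; SpawnArrow attaches a collision-free arrow to the mesh's Arrow socket.
; FaShe detaches it and activates projectile movement along the user's forward vector with scaled speed and collision.
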(event `self.ReceiveBeginPlay`
  (`parent.ReceiveBeginPlay`)
  (set `self.AMPianDuan` (`|MakeArray` "PuTong" "XuLi" "XuLiEnd" :!type "Name")))

(event `GongJiAM`
  (params (KeyIn :type Boolean))
  (bind _user (`self.User`))
  (`/Engine/EditorBlueprintResources/StandardMacros.DoOnce` false :!label _label
    (:`Completed`
      (`/Game/RPG/Blueprints/Player/BP_PlayerBase.XiuZheng` _user 1000.0)
      (`|PlayMontage` (`Character.Mesh` _user) "/Game/RPG/Animation/GongJi/AM_Gong_A.AM_Gong_A" 1.0 0.0 (`|GetArrayItem` (`self.AMPianDuan`) (`self.NowPianDuanIndex`))
        (:`then`
          (`self.DisableInput` (`self.User`) (`GameplayStatics.GetPlayerController` 0)))
        (:`OnCompleted`
          (set `self.NowPianDuanIndex` 0)
          (`self.EnableInput` (`self.User`) (`GameplayStatics.GetPlayerController` 0))
          (`self.Reset`))))))

(event `Reset`
  (goto _label :!via `Reset`))

(event `EnhancedInput|/Game/RPG/Input/IA/IA_GongJi`
  (params (ActionValue :type Boolean) (ElapsedSeconds :type "Float (double-precision)") (TriggeredSeconds :type "Float (double-precision)") (InputAction :type "InputAction Object Reference" :default "/Game/RPG/Input/IA/IA_GongJi.IA_GongJi"))
  (:`Triggered`
    (`self.GongJiAM` false)))

(fn `EndGongJi`
  (`parent.EndGongJi`)
  (`/Game/RPG/Blueprints/Player/BP_PlayerBase.XiuZheng` (`self.User`) 800.0))

(fn `Fa She`
  (bind _arrow (`self.Arrow`))
  (bind _projectilemovement (`/Game/RPG/Blueprints/WuQi/WuQiBlueprint/BP_Arrow.ProjectileMovement` _arrow))
  (`/Engine/EditorBlueprintResources/StandardMacros.IsValid` _arrow
    (:`Is Valid`
      (`self.K2_DetachFromActor` _arrow "KeepWorld" "KeepWorld" "KeepWorld")
      (set `MovementComponent.Velocity` (* (* (`KismetMathLibrary.VSize` (`MovementComponent.Velocity` _projectilemovement)) (`self.ArrowSpeed`)) (`self.GetActorForwardVector` (`self.User`))) _projectilemovement)
      (`ActorComponent.Activate` _projectilemovement true)
      (`self.SetActorEnableCollision` (`self.Arrow`) true))))

(fn `Spawn Arrow`
  (bind _returnvalue (`|SpawnActorFromClass` "/Game/RPG/Blueprints/WuQi/WuQiBlueprint/BP_Arrow.BP_Arrow_C" (`KismetMathLibrary.MakeTransform` (0.0 0.0 0.0)) "Undefined" "MultiplyWithRoot" null "NewEnumerator1" "NewEnumerator0" null))
  (bind _output_get (set `self.Arrow` _returnvalue))
  (`self.SetActorEnableCollision` _output_get false)
  (set `/Game/RPG/Blueprints/WuQi/BP_WuQiBase.User` (`self.User`) _output_get)
  (set `/Game/RPG/Blueprints/WuQi/WuQiBlueprint/BP_Arrow.AsGong` self _output_get)
  (`self.K2_AttachToComponent` _output_get (`Character.Mesh` (`self.User`)) "Arrow" "SnapToTarget" "SnapToTarget" "SnapToTarget" true))

(fn `StartGongJi`
  (`parent.StartGongJi`)
  (`self.Reset`))

(fn `UserConstructionScript`
  (`parent.UserConstructionScript`))