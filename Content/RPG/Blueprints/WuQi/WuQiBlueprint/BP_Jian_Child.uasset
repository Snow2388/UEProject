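; Sword (Jian) child weapon that performs a combo melee attack for its user and damages enemies it hits.
; The attack input passes a DoOnce gate, calls XiuZheng on the user, disables their input and plays the current montage section.
; StartGongJi advances the section index and reopens the gate for chaining, while montage completion resets the combo.
; GongJi component overlaps call BeAttacked on BP_EnemyBase targets with the sword's base damage.
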(event `self.ReceiveBeginPlay`
  (`parent.ReceiveBeginPlay`)
  (set `self.AMPianDuan` (`|MakeArray` "0" "1" "2" "3" "4" :!type "Name")))

(event `GongJiAM`
  (bind _user (`self.User`))
  (set `PrimitiveComponent.bGenerateOverlapEvents` true (`self.GongJi`))
  (`/Engine/EditorBlueprintResources/StandardMacros.DoOnce` false :!label _label
    (:`Completed`
      (`/Game/RPG/Blueprints/Player/BP_PlayerBase.XiuZheng` _user 200.0)
      (`|PlayMontage` (`Character.Mesh` _user) "/Game/RPG/Animation/GongJi/AM_Jian_A.AM_Jian_A" 1.0 0.0 (`|GetArrayItem` (`self.AMPianDuan`) (`self.NowPianDuanIndex`))
        (:`then`
          (`self.DisableInput` (`self.User`) (`GameplayStatics.GetPlayerController` 0)))
        (:`OnCompleted`
          (set `self.NowPianDuanIndex` 0)
          (`self.EnableInput` (`self.User`) (`GameplayStatics.GetPlayerController` 0))
          (`self.Reset`)
          (set `PrimitiveComponent.bGenerateOverlapEvents` false (`self.GongJi`)))))))

(event `Reset`
  (goto _label :!via `Reset`))

(event `EnhancedInput|/Game/RPG/Input/IA/IA_GongJi`
  (params (ActionValue :type Boolean) (ElapsedSeconds :type "Float (double-precision)") (TriggeredSeconds :type "Float (double-precision)") (InputAction :type "InputAction Object Reference" :default "/Game/RPG/Input/IA/IA_GongJi.IA_GongJi"))
  (:`Triggered`
    (`self.GongJiAM`)))

(event `self.GongJi.OnComponentBeginOverlap`
  (params (OverlappedComponent :type "PrimitiveComponent Object Reference") (OtherActor :type "Actor Object Reference") (OtherComp :type "PrimitiveComponent Object Reference") (OtherBodyIndex :type Integer) (bFromSweep :type Boolean) (SweepResult :type "HitResult Structure (by ref)"))
  (bind _user (`self.User`)
    (:`then`
      (bind _asbp_enemy_base (cast `/Game/RPG/Blueprints/Enemy/BP_EnemyBase` OtherActor))
      (`/Game/RPG/Blueprints/Interface/IF_BeAttacked.BeAttacked` _asbp_enemy_base (`self.Base Damage_Jian`) _user self))
    (:`else`)))

(fn `EndGongJi`
  (`parent.EndGongJi`))

(fn `StartGongJi`
  (`parent.StartGongJi`)
  (bind _result (`/Engine/EditorBlueprintResources/StandardMacros.IncrementInt` (`self.NowPianDuanIndex`))
    (:`  `
      (if (not (`KismetArrayLibrary.Array_IsValidIndex` (`self.AMPianDuan`) _result))
        (set `self.NowPianDuanIndex` 0))
      (`self.Reset`))))

(fn `UserConstructionScript`
  (`parent.UserConstructionScript`))