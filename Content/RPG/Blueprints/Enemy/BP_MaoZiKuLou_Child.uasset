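; Child enemy Blueprint for the MaoZiKuLou (hat skeleton) in the RPG, configuring an inherited enemy for this variant.
; On BeginPlay it runs the parent logic, then sets attack montage section names, attack and hit-reaction montages, death animations, health and the TimeChouHeng timer value (likely aggro time).
; It adds no behavior of its own, as overlap and tick events are disabled stubs and construction only calls the parent.
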(event `self.ReceiveBeginPlay`
  (`parent.ReceiveBeginPlay`)
  (set `self.AMPianDuan_GongJi` (`|MakeArray` "0" "1" "2" "3" "4" "5" "6" "7" :!type "Name"))
  (set `self.DieAnima` (`|MakeArray` "/Game/CityofBrass_Enemies/Meshes/Enemy/Corpse/animation/Corpse_Alert_Death.Corpse_Alert_Death" "/Game/CityofBrass_Enemies/Meshes/Enemy/Corpse/animation/Corpse_Alert_Death2.Corpse_Alert_Death2" "/Game/CityofBrass_Enemies/Meshes/Enemy/Corpse/animation/Corpse_Alert_Death3.Corpse_Alert_Death3" :!type "AnimSequence Object Reference"))
  (set `self.AM_GongJi` "/Game/RPG/Animation/GongJi/Enemy/AM_MaoZiKuLou_A.AM_MaoZiKuLou_A")
  (set `self.AM_BeAttacked` "/Game/RPG/Animation/GongJi/Enemy/AM_MaoZiKuLou_BeAttacked.AM_MaoZiKuLou_BeAttacked")
  (bind _output_get (set `self.MaxHP` 100.0))
  (set `self.NowHP` _output_get)
  (set `self.Time_ChouHeng` 6.0))

(fn `UserConstructionScript`
  (`parent.UserConstructionScript`))