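; Base enemy for the RPG with patrol, chase, attack, hit and death behavior, driven by a state enum and PawnSensing.
; It roams random navmesh points until it sees a player, then widens its vision, chases and plays random attack montage sections.
; A retriggerable delay drops aggro after lost sight, restoring health and patrol.
; Hits show the health widget and play a reaction; zero health plays a death animation and destroys it.
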(event `self.ReceiveBeginPlay`
  ;[1 1 1] 开始游戏时巡逻
  (bind _asumg_enemy_hp (cast `/Game/RPG/UMG/UMG_EnemyHP` (`WidgetComponent.GetWidget` (`self.UMG_HPComponent`))))
  (set `/Game/RPG/UMG/UMG_EnemyHP.EnemyAs` self _asumg_enemy_hp)
  (`KismetSystemLibrary.Delay` 2.0)
  (set `self.State` "NewEnumerator0")
  (`self.AutoMove`))

(event `AutoMove`
  ;[1 1 1] 自动巡逻
  (if (`|EnumEquality` (`self.State`) "NewEnumerator0")
    (`|AIMoveTo` self (`NavigationSystemV1.K2_GetRandomReachablePointInRadius` (`NavigationSystemV1.GetNavigationSystem`) (`self.K2_GetActorLocation`) 500.0 null null) null 50.0
      (:`OnSuccess`
        _)
      (:`OnFail`
        _))
    (`KismetSystemLibrary.Delay` (`KismetMathLibrary.RandomFloatInRange` 2.0 5.0))
    (`self.AutoMove`)))

(event `self.PawnSensing.OnSeePawn`
  (params (Pawn :type "Pawn Object Reference"))
  ;[1 1 1] 追击玩家，追击状态超过‘Time_ChouHeng’未检测到玩家，仇恨值清空，转为巡逻状态
  (bind _asbp_player_base (cast `/Game/RPG/Blueprints/Player/BP_PlayerBase` Pawn))
  (`PawnSensingComponent.SetPeripheralVisionAngle` (`self.PawnSensing`) 180.0)
  (set `self.State` "NewEnumerator1")
  (`self.ZhuiJi` _asbp_player_base)
  (`KismetSystemLibrary.RetriggerableDelay` (`self.Time_ChouHeng`))
  (`self.Again_XunLuo`))

(event `ZhuiJi`
  (params (Player :type "/Game/RPG/Blueprints/Player/BP_PlayerBase Object Reference"))
  ;[1 1 1] 追击玩家，追击状态超过‘Time_ChouHeng’未检测到玩家，仇恨值清空，转为巡逻状态
  (bind _output_get (set `self.ChouHengPlayer` Player))
  (`|AIMoveTo` self (0.0 0.0 0.0) _output_get 0.0
    (:`OnSuccess`
      (`self.GongJi`))))

(event `Again_XunLuo`
  ;[1 1 1] 追击玩家，追击状态超过‘Time_ChouHeng’未检测到玩家，仇恨值清空，转为巡逻状态
  (set `self.ChouHengPlayer` null)
  (set `self.NowHP` (`self.MaxHP`))
  (if (not (`|EnumEquality` (`self.State`) "NewEnumerator2"))
    (set `self.State` "NewEnumerator0")
    (`PawnSensingComponent.SetPeripheralVisionAngle` (`self.PawnSensing`) 45.0)
    (`self.AutoMove`)
    (`SceneComponent.SetVisibility` (`self.UMG_HPComponent`) false false)))

(event `GongJi`
  ;[1 1 1] 攻击
  (`PawnSensingComponent.SetSensingUpdatesEnabled` (`self.PawnSensing`) false)
  (`/Engine/EditorBlueprintResources/StandardMacros.DoOnce` false :!label _label
    (:`Completed`
      (bind _am_gongji (`self.AM_GongJi`)
        (:`then`
          (`|PlayMontage` (`self.Mesh`) _am_gongji 1.0 0.0 (`KismetArrayLibrary.Array_Random` (`self.AMPianDuan_GongJi`))
            (:`OnCompleted`
              (`self.Reset`)
              (`PawnSensingComponent.SetSensingUpdatesEnabled` (`self.PawnSensing`) true))))
        (:`else`)))))

(event `Reset`
  ;[1 1 1] 攻击
  (goto _label :!via `Reset`))

(event `/Game/RPG/Blueprints/Interface/IF_BeAttacked.BeAttacked`
  (params (BaseDamage :type "Float (double-precision)") (DamagePlayer :type "/Game/RPG/Blueprints/Player/BP_PlayerBase Object Reference") (WuQi :type "/Game/RPG/Blueprints/WuQi/BP_WuQiBase Object Reference"))
  (bind _nowhp (`self.NowHP`))
  ;[1 1 1] 被攻击
  (set `self.ChouHengPlayer` DamagePlayer)
  (`MovementComponent.StopMovementImmediately` (`self.CharacterMovement`))
  (`SceneComponent.SetVisibility` (`self.UMG_HPComponent`) true false)
  (`PawnSensingComponent.SetSensingUpdatesEnabled` (`self.PawnSensing`) false)
  (set `self.State` "NewEnumerator2")
  (if (> _nowhp 0.0)
    (set `self.NowHP` (`KismetMathLibrary.FClamp` (- _nowhp BaseDamage) 0.0 99999.0))
    (if (== (`self.NowHP`) 0.0)
      (`self.Die`)
      (else
        (bind _am_beattacked (`self.AM_BeAttacked`)
          (:`then`
            (`|PlayMontage` (`self.Mesh`) _am_beattacked
              (:`OnCompleted`
                (`PawnSensingComponent.SetSensingUpdatesEnabled` (`self.PawnSensing`) true)
                (`self.Reset`)
                (set `self.State` "NewEnumerator0"))))
          (:`else`))))))

(event `Die`
  ;[1 1 1] 死亡
  (set `self.State` "NewEnumerator3")
  (`CharacterMovementComponent.DisableMovement` (`self.CharacterMovement`))
  (`SceneComponent.SetVisibility` (`self.UMG_HPComponent`) false false)
  (`PawnSensingComponent.SetSensingUpdatesEnabled` (`self.PawnSensing`) false)
  (`self.SetActorEnableCollision` false)
  (`SkeletalMeshComponent.PlayAnimation` (`self.Mesh`) (`KismetArrayLibrary.Array_Random` (`self.DieAnima`)) false)
  (`KismetSystemLibrary.Delay` 3.0)
  (`self.K2_DestroyActor`))

(fn `UserConstructionScript`)